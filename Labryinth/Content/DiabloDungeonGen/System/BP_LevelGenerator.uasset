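; Dungeon level generator actor that builds and spawns a random tile layout on BeginPlay.
; GenerateTileLayout random-walks from a start tile, picking unoccupied cells via LocationToSeek offsets and storing each in the TileLayout map.
; SpawnTileLayout then spawns an actor per map key, scaling grid coordinates by TileSize.
; GetTileClass currently returns BP_StartTile for every type, and IsTileUsed returns true for free cells, despite its name.
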(event EventBeginPlay
  (Generation|GenerateTileLayout)
  (Generation|SpawnTileLayout))

(fn ConstructionScript)

(fn SpawnTile
  (params (TileToSpawn :type BP%20Tile%20Class%20Reference) (SpawnTransform :type Transform))
  (Game|SpawnActorfromClass TileToSpawn SpawnTransform "AlwaysSpawn" 0 0))

(fn GenerateTileLayout
  (Utilities|Map|Add :TargetMap (Variables|Default|GetTileLayout) :Value (Utilities|Struct|MakeSTileInformation "NewEnumerator1" (LocalVariables|GetemptyConnections)))
  (for _index (range 1 (Math|Float|Truncate (Variables|Default|GetValueAmount)))
    (LocalVariables|SetfoundLocation (Rules|FindRandomNextLocation (LocalVariables|GetpreviousLocation)))
    (Utilities|Map|Add (Variables|Default|GetTileLayout) (LocalVariables|GetfoundLocation) (Utilities|Struct|MakeSTileInformation "NewEnumerator0" (LocalVariables|GetemptyConnections)))
    (bind _output_get (LocalVariables|SetpreviousLocation (LocalVariables|GetfoundLocation)))
    (CallFunction|Debug false "Found Location:" (Utilities|String|ToString(Vector2d) _output_get) "(R=0.139947,G=0.366653,B=0.502604,A=1.000000)")))

(fn SpawnTileLayout
  (bind _tilelayout (Variables|Default|GetTileLayout))
  (bind _keys (Utilities|Map|Keys _tilelayout))
  (for _array_element _keys
    (Generation|SpawnTile (Utility|GetTileClass (.Type (Utilities|Struct|BreakSTileInformation (.Value (Utilities|Map|Find _tilelayout _array_element))))) (Utility|GetTileLocation _array_element))))

(fn GetTileClass
  (params (InTileType :type ETileType%20Enum :default "NewEnumerator0"))
  (return "/Game/DiabloDungeonGen/Tile/BP_StartTile.BP_StartTile_C"))

(fn GetTileLocation
  (params (InTileLocation :type Vector%202D%20Structure))
  (bind (_x _y) (Math|Vector2D|BreakVector2D InTileLocation))
  (bind _tilesize (Variables|Default|GetTileSize))
  (bind (_x_2 _y_2) (Math|Vector|BreakVector _tilesize))
  (return (Math|Transform|MakeTransform (Math|Vector|MakeVector (* _x _x_2) (* _y _y_2) 0.0))))

(fn FindRandomNextLocation
  (params (StartingLocation :type Vector%202D%20Structure))
  (bind _validlocations (LocalVariables|GetvalidLocations))
  (for _array_element (LocalVariables|GetlocationToSeek)
    (if (not (not (Utility|IsTileUsed (+ StartingLocation _array_element))))
      (Utilities|Array|Add (LocalVariables|GetvalidLocations) (+ StartingLocation _array_element))))
  (return (Utilities|Array|Get(acopy) _validlocations (Math|Random|RandomIntegerinRange 0 (Utilities|Array|LastIndex _validlocations)))))

(fn IsTileUsed
  (params (AtLocation :type Vector%202D%20Structure))
  (return (not (.ReturnValue (Utilities|Map|Find (Variables|Default|GetTileLayout) AtLocation)))))

(fn Debug
  (params (Enabled :type Boolean) (Intext :type String) (Append :type String) (TextColor :type Linear%20Color%20Structure))
  (if Enabled
    (Development|PrintString (Utilities|String|Append Intext Append) true true TextColor)))