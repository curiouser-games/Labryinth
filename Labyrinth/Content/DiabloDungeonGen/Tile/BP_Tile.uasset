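; BP_Tile is a dungeon generation tile that opens its sides to match its connections.
; On BeginPlay, GenerateConnectors walks the TileConnection map of direction to boolean.
; For each true entry, it shows that side's North, South, East or West component and destroys the matching wall component.
; False entries are left untouched, and the Random direction maps to no component.
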(event EventBeginPlay
  (CallFunction|GenerateConnectors))

(fn ConstructionScript)

(fn GenerateConnectors
  (bind _tileconnection (Variables|Metrics|GetTileConnection))
  (bind _keys (Utilities|Map|Keys _tileconnection))
  (for _array_element _keys
    (if (.Value (Utilities|Map|Find _tileconnection _array_element))
      (Rendering|SetVisibility (Utilities|Select :Index _array_element :NewEnumerator0 (Variables|Default|GetNorth) :NewEnumerator1 (Variables|Default|GetSouth) :NewEnumerator2 (Variables|Default|GetEast) :NewEnumerator3 (Variables|Default|GetWest) :NewEnumerator4 0) (.Value (Utilities|Map|Find _tileconnection _array_element)) false)
      (Development|SetHiddeninGame (Utilities|Select :Index _array_element :NewEnumerator0 (Variables|Default|GetNorth) :NewEnumerator1 (Variables|Default|GetSouth) :NewEnumerator2 (Variables|Default|GetEast) :NewEnumerator3 (Variables|Default|GetWest) :NewEnumerator4 0) (not (.Value (Utilities|Map|Find _tileconnection _array_element))) false)
      (Components|DestroyComponent (Utilities|Select :Index _array_element :NewEnumerator0 (Variables|Default|GetNorthernWall) :NewEnumerator1 (Variables|Default|GetSouthernWall) :NewEnumerator2 (Variables|Default|GetEasternWall) :NewEnumerator3 (Variables|Default|GetWesternWall) :NewEnumerator4 0)))))