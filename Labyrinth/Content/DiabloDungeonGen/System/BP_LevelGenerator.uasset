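; Procedural dungeon level generator actor that builds a grid of tile actors on BeginPlay and regenerates it on a debug key press.
; A random walk from the start tile fills a location-to-type-and-connections map, then passes add side tiles, extra connections and replacement tiles.
; Each cell spawns a tile class matched on connection defaults, attached to the generator.
; End-tile placement is unwired and the steps-to-start pass is unfinished.
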(event EventBeginPlay
  (System|GenerateLevel))

(event Input|KeyboardEvents|Add
  (params (Key :type Key%20Structure))
  (:Pressed
    (System|GenerateLevel)))

(fn ConstructionScript)

(fn SpawnTile
  (params (TileToSpawn :type BP%20Tile%20Class%20Reference) (SpawnTransform :type Transform) (TileType :type ETileType%20Enum :default "NewEnumerator0"))
  (bind _returnvalue (Game|SpawnActorfromClass TileToSpawn SpawnTransform "AlwaysSpawn" 0 TileType 0 0))
  ;[1 1 1] makes sure i can rotate tile and all tiles remain rotated
  (Transformation|AttachActorToActor _returnvalue self "None" "KeepRelative" "SnapToTarget" "KeepRelative" true)
  ;[1 1 1] we're keeping track of the tiles spawned to remove them later
  (Utilities|Array|Add (Variables|References|GetTiles) 0))

(fn GenerateTileLayout
  ;[1 1 1] start tile
  (Layout|AddStartTiletoLayout)
  (for _index (range 1 (Variables|Metrics|GetTileAmount))
    ;[1 1 1] generic tiles
    (if (not (Utility|ShouldStepBack _index))
      (bind (_succesfullyadded _foundlocation) (Layout|TryAddTiletoLayout (LocalVariables|GetpreviousLocation) (select (== (Utilities|Map|Length (Variables|References|GetTileLayout)) 1) "NewEnumerator1" "NewEnumerator4") "NewEnumerator0"))
      ;[1 1 1] Random is returned if we are not finding any sport
      (if _succesfullyadded
        (LocalVariables|SetpreviousLocation _foundlocation)
        (else
          (bind _foundlocation_2 (Layout|StepBack "NewEnumerator4" "NewEnumerator0"))
          ;[1 1 1] if manage to, our new tile is now previous location
          (LocalVariables|SetpreviousLocation _foundlocation_2)))
      (else
        (Layout|StepBack "NewEnumerator0" "NewEnumerator0")))))

(fn SpawnTileLayout
  (bind _tilelayout (Variables|References|GetTileLayout))
  (bind _keys (Utilities|Map|Keys _tilelayout))
  (for _array_element _keys
    (System|SpawnTile (Layout|GetTileClass (.Type (Utilities|Struct|BreakSTileInformation (.Value (Utilities|Map|Find _tilelayout _array_element)))) (.Directions (Utilities|Struct|BreakSTileInformation (.Value (Utilities|Map|Find _tilelayout _array_element)))) _array_element) (Utility|GetTileLocation _array_element) (.Type (Utilities|Struct|BreakSTileInformation (.Value (Utilities|Map|Find _tilelayout _array_element)))))))

(fn GetTileClass
  (params (InTileType :type ETileType%20Enum :default "NewEnumerator0") (InDirections :type Map%20of%20ECardinalPoint%20Enums%20to%20Booleans :default "NewEnumerator0") (AtLocation :type Vector%202D%20Structure))
  (if (Utilities|Enum|Equal(Enum) InTileType "NewEnumerator1")
    (return "/Game/DiabloDungeonGen/Tile/BP_StartTile.BP_StartTile_C")
    (elif (or (Utilities|Enum|Equal(Enum) InTileType "NewEnumerator0") (Utilities|Enum|Equal(Enum) InTileType "NewEnumerator3"))
      (bind _output (Utility|FindRandomValidTile (Variables|Metrics|GetGenericTileList) InDirections))
      (return _output)
      (elif (Utilities|Enum|Equal(Enum) InTileType "NewEnumerator2")
        (bind _output_2 (Utility|FindRandomValidTile (Variables|Metrics|GetEndTileList) InDirections))
        (return _output_2)
        (elif (Utilities|Enum|Equal(Enum) InTileType "NewEnumerator4")
          (return (.Value (Utilities|Map|Find (Variables|References|GetReplacedTileClass) AtLocation)))
          (else
            (return "/Game/DiabloDungeonGen/Tile/BP_StartTile.BP_StartTile_C")))))))

(fn GetTileLocation
  (params (InTileLocation :type Vector%202D%20Structure))
  (bind (_x _y) (Math|Vector2D|BreakVector2D InTileLocation))
  (bind _tilesize (Variables|Metrics|GetTileSize))
  (bind (_x_2 _y_2) (Math|Vector|BreakVector _tilesize))
  (return (Math|Transform|MakeTransform (Math|Vector|MakeVector (* _x _x_2) (* _y _y_2) 0.0))))

(fn FindRandomNextLocation
  (params (StartingLocation :type Vector%202D%20Structure) (WantedDirection :type ECardinalPoint%20Enum :default "NewEnumerator0"))
  (bind _locationtoseeknew (LocalVariables|GetlocationToSeekNew))
  (LocalVariables|SettempStartingLocation StartingLocation)
  (if (Utilities|Enum|Equal(Enum) WantedDirection "NewEnumerator4")
    (bind _keys (Utilities|Map|Keys (LocalVariables|GetlocationToSeekNew)))
    (for _array_element _keys
      ;[1 1 1] SWITCH THIS TO MAKE WORK FOR SOME REASON
      (if (not (Utility|IsLocationUsed (+ (LocalVariables|GettempStartingLocation) (.Value (Utilities|Map|Find (LocalVariables|GetlocationToSeekNew) _array_element)))))
        (Utilities|Map|Remove (LocalVariables|GetlocationToSeekNew) _array_element)))
    (bind _keys_2 (Utilities|Map|Keys _locationtoseeknew :!label _label))
    (if (> (Utilities|Array|Length _keys_2) 0)
      (bind _output_get (LocalVariables|SetrandomizedResult (Utilities|Array|Get(acopy) _keys_2 (Math|Random|RandomIntegerinRange 0 (Utilities|Array|LastIndex _keys_2)))))
      (LocalVariables|SettempFoundLocation (+ (.Value (Utilities|Map|Find _locationtoseeknew _output_get)) (LocalVariables|GettempStartingLocation)))
      (if (.Value (Utilities|Map|Find (.Directions (Utilities|Struct|BreakSTileInformation (.Value (Utilities|Map|Find (Variables|References|GetTileLayout) (LocalVariables|GettempStartingLocation))))) (Utility|WhereAmIComingfrom (LocalVariables|GettempStartingLocation) (LocalVariables|GettempFoundLocation))))
        (if (== (Variables|References|GetCorridorsSpawned) (Variables|Metrics|GetMaxCorridorsInARow))
          (Utilities|Map|Remove (LocalVariables|GetlocationToSeekNew) (LocalVariables|GetrandomizedResult))
          (goto _label)
          (else
            (Math|Integer|IncrementInt (Variables|References|GetCorridorsSpawned)
              (:%20%20
                _))))
        (else
          (Variables|References|SetCorridorsSpawned 0)))
      (return (LocalVariables|GettempFoundLocation) (LocalVariables|GetrandomizedResult))
      (else
        (return "" "NewEnumerator4")))
    (else
      (return (.Value (Utilities|Map|Find (LocalVariables|GetlocationToSeekNew) WantedDirection)) WantedDirection))))

(fn IsLocationUsed
  (params (AtLocation :type Vector%202D%20Structure))
  (return (not (.ReturnValue (Utilities|Map|Find (Variables|References|GetTileLayout) AtLocation)))))

(fn Debug
  (params (Enabled :type Boolean) (Intext :type String) (Append :type String) (TextColor :type Linear%20Color%20Structure))
  (if Enabled
    (Development|PrintString (Utilities|String|Append Intext Append) true true TextColor)))

(fn ConnectTiles
  (params (InTile :type Vector%202D%20Structure) (ToOtherTile :type Vector%202D%20Structure) (FromCardinal :type ECardinalPoint%20Enum :default "NewEnumerator0"))
  (Layout|SetConnectionEnabled InTile (Utility|RevertCardinal FromCardinal) true)
  (Layout|SetConnectionEnabled ToOtherTile FromCardinal true))

(fn SetConnectionEnabled
  (params (InTile :type Vector%202D%20Structure) (ToCardinalPoint :type ECardinalPoint%20Enum :default "NewEnumerator0") (Enabled :type Boolean))
  (bind _tilelayout (Variables|References|GetTileLayout))
  (bind (_value _returnvalue) (Utilities|Map|Find _tilelayout InTile))
  (bind (_type _directions) (Utilities|Struct|BreakSTileInformation _value))
  (if _returnvalue
    (LocalVariables|SettempDirection _directions)
    (Utilities|Map|Add (LocalVariables|GettempDirection) ToCardinalPoint Enabled)
    (Utilities|Map|Add (Variables|References|GetTileLayout) InTile (Utilities|Struct|MakeSTileInformation _type (LocalVariables|GettempDirection)))))

(fn AreConnectionsEqual
  (params (Connection_1 :type Map%20of%20Bytes%20to%20Booleans) (Connection_2 :type Map%20of%20Bytes%20to%20Booleans))
  (LocalVariables|SetnotEqual false)
  (bind _keys (Utilities|Map|Keys Connection_1))
  (for _array_element _keys
    (if (.ReturnValue (Utilities|Map|Find Connection_2 _array_element))
      (if (not (Math|Boolean|Equal(Boolean) (.Value (Utilities|Map|Find Connection_2 _array_element)) (.Value (Utilities|Map|Find Connection_1 _array_element))))
        (LocalVariables|SetnotEqual true))
      (else
        (LocalVariables|SetnotEqual (.Value (Utilities|Map|Find Connection_1 _array_element))))))
  (return (not (LocalVariables|GetnotEqual))))

(fn RevertCardinal
  (params (InCardinal :type ECardinalPoint%20Enum :default "NewEnumerator0"))
  (return (Utilities|Select :Index InCardinal :NewEnumerator0 "NewEnumerator1" :NewEnumerator1 "NewEnumerator0" :NewEnumerator2 "NewEnumerator3" :NewEnumerator3 "NewEnumerator2" :NewEnumerator4 "NewEnumerator4")))

(fn AreConnectionsMatching
  (params (InConnections :type Map%20of%20ECardinalPoint%20Enums%20to%20Booleans :default "NewEnumerator0") (AgainstConnections :type Map%20of%20ECardinalPoint%20Enums%20to%20Booleans :default "NewEnumerator0"))
  (LocalVariables|SetbTempValidTiles true)
  (bind _keys (Utilities|Map|Keys InConnections))
  (bind _array_element (Utilities|Array|ForEachLoopwithBreak _keys :!label _label)
    (:LoopBody
      (if (Math|Boolean|NotEqual(Boolean) (.Value (Utilities|Map|Find InConnections _array_element)) (.Value (Utilities|Map|Find AgainstConnections _array_element)))
        (LocalVariables|SetbTempValidTiles false)
        (goto _label Break)))
    (:Completed
      (return (LocalVariables|GetbTempValidTiles)))))

(fn FindRandomValidTile
  (params (Array :type Array%20of%20BP%20Tile%20Class%20References) (InConnections :type Map%20of%20ECardinalPoint%20Enums%20to%20Booleans :default "NewEnumerator0"))
  (bind _validtiles (LocalVariables|GetvalidTiles))
  (for _array_element Array
    (if (Utility|AreConnectionsMatching InConnections (.TileConnection (Utilities|GetClassDefaults _array_element)))
      (Utilities|Array|Add (LocalVariables|GetvalidTiles) _array_element)))
  (return (Utilities|Array|Get(acopy) _validtiles (Math|Random|RandomIntegerinRange 0 (Utilities|Array|LastIndex _validtiles)))))

(fn GenerateExtraConnections
  (bind _tilelayout (Variables|References|GetTileLayout))
  (bind _keys (Utilities|Map|Keys _tilelayout))
  (bind _array_element (Utilities|Array|ForEachLoopwithBreak _keys :!label _label)
    (:LoopBody
      (if (Utilities|Enum|Equal(Enum) (.Type (Utilities|Struct|BreakSTileInformation (.Value (Utilities|Map|Find _tilelayout _array_element)))) "NewEnumerator0")
        (if (and (Variables|Metrics|GetbConnectAdditionalTiles) (Utilities|Enum|Equal(Enum) (.Type (Utilities|Struct|BreakSTileInformation (.Value (Utilities|Map|Find _tilelayout _array_element)))) "NewEnumerator3"))
          (bind _array_element_2 (Utilities|Array|ForEachLoopwithBreak (Utility|GetLocationsAround _array_element) :!label _label_2)
            (:LoopBody
              (if (and (Utility|IsLocationUsed _array_element_2) (Utilities|Enum|Equal(Enum) (.Type (Utilities|Struct|BreakSTileInformation (.Value (Utilities|Map|Find (Variables|References|GetTileLayout) _array_element_2)))) "NewEnumerator0"))
                (if (not (Utility|AreTilesConnected _array_element_2 _array_element))
                  (Layout|ConnectTiles _array_element_2 _array_element (Utility|WhereAmIComingfrom _array_element_2 _array_element) :!label _label_3)
                  (Math|Integer|DecrementInt (Variables|References|GetRemainingConnections)
                    (:%20%20
                      (if (<= 0 (Variables|References|GetRemainingConnections))
                        (goto _label_2 Break))))
                  (elif (and (Variables|Metrics|GetbConnectAdditionalTiles) (Utilities|Enum|Equal(Enum) (.Type (Utilities|Struct|BreakSTileInformation (.Value (Utilities|Map|Find (Variables|References|GetTileLayout) _array_element_2)))) "NewEnumerator3"))
                    (goto _label_3)))))
            (:Completed
              (if (<= 0 (Variables|References|GetRemainingConnections))
                (goto _label Break)))))))))

(fn GetLocationsAround
  (params (InLocation :type Vector%202D%20Structure))
  (Utilities|Array|Add (LocalVariables|GettempLocations) (+ InLocation "(X=1.000000,Y=0.000000)"))
  (Utilities|Array|Add (LocalVariables|GettempLocations) (+ InLocation "(X=-1.000000,Y=0.000000)"))
  (Utilities|Array|Add (LocalVariables|GettempLocations) (+ InLocation "(X=0.000000,Y=1.000000)"))
  (Utilities|Array|Add (LocalVariables|GettempLocations) (+ InLocation "(X=0.000000,Y=-1.000000)"))
  (return (LocalVariables|GettempLocations)))

(fn AreTilesConnected
  (params (InTile :type Vector%202D%20Structure) (InSecondTile :type Vector%202D%20Structure))
  (return (.Value (Utilities|Map|Find (.Directions (Utilities|Struct|BreakSTileInformation (.Value (Utilities|Map|Find (Variables|References|GetTileLayout) InSecondTile)))) (Utility|WhereAmIComingfrom InTile InSecondTile)))))

(fn WhereAmIComingfrom
  (params (FromTile :type Vector%202D%20Structure) (ToTile :type Vector%202D%20Structure))
  (bind _returnvalue (- FromTile ToTile))
  (bind (_x _y) (Math|Vector2D|BreakVector2D _returnvalue))
  (if (and (> _x 0.0) (== _y 0.0))
    (return "NewEnumerator0")
    (elif (and (< _x 0.0) (== _y 0.0))
      (return "NewEnumerator1")
      (elif (and (== _x 0.0) (> _y 0.0))
        (return "NewEnumerator2")
        (elif (and (== _x 0.0) (< _y 0.0))
          (return "NewEnumerator3")
          (else
            (return "NewEnumerator4")))))))

(fn GenerateLevel
  (System|ResetLevel)
  (Generation|GenerateTileLayout)
  (if (Variables|Metrics|GetbConnectAdditionalTiles)
    (Generation|GenerateAdditionalTileLayout)
    (Generation|GenerateExtraConnections)
    (else
      (Generation|GenerateExtraConnections)
      (Generation|GenerateAdditionalTileLayout)))
  (Generation|GenerateReplacementTileLayout)
  (Generation|CalculateStepstoStart)
  (Generation|SpawnTileLayout))

(fn ResetLevel
  (bind _arrayelement (Utilities|Array|ReverseforEachLoop (Variables|References|GetTiles))
    (:LoopBody
      (Transformation|DetachFromActor _arrayelement "KeepRelative" "KeepRelative" "KeepRelative")
      (Actor|DestroyActor _arrayelement))
    (:Completed
      (Variables|References|SetRemainingConnections (Variables|Metrics|GetExtraConnections))
      (Utilities|Map|Clear (Variables|References|GetTileLayout))
      (Utilities|Array|Clear (Variables|References|GetTiles))
      (Variables|References|SetCorridorsSpawned 0))))

(fn GenerateAdditionalTileLayout
  ;[1 1 1] if we will be looping without randomizing, we would get only additional tiles at the beginning of the level
  (bind _keys (Utilities|Map|Keys (Variables|References|GetTileLayout)))
  (bind _output_get (LocalVariables|SettempLocations _keys))
  (Utilities|Array|Shuffle _output_get)
  (if (> (Variables|Metrics|GetAdditionalTileAmount) 0)
    (for _index (range 1 (Variables|Metrics|GetAdditionalTileAmount))
      ;[1 1 1] each time we loop we make sure our "found location" checker is reset
      (LocalVariables|SetbFoundLocation false)
      ;[1 1 1] we get each generic tile in the level, then we get each tile around this and we check if these tiles are used
      (bind (_array_element _array_index) (Utilities|Array|ForEachLoopwithBreak (LocalVariables|GettempLocations) :!label _label)
        (:LoopBody
          (if (Utilities|Enum|Equal(Enum) (.Type (Utilities|Struct|BreakSTileInformation (.Value (Utilities|Map|Find (Variables|References|GetTileLayout) _array_element)))) "NewEnumerator0")
            (bind _array_element_2 (Utilities|Array|ForEachLoopwithBreak (Utility|GetLocationsAround _array_element) :!label _label_2)
              (:LoopBody
                (if (not (Utility|IsLocationUsed _array_element_2))
                  ;[1 1 1] if tiles not used generate additional tile and we remove the generic tile we added
                  (LocalVariables|SettempLocToRemove _array_index)
                  (Layout|AddTiletoLayout _array_element_2 "NewEnumerator3" _array_element)
                  (LocalVariables|SetbFoundLocation true)
                  (goto _label_2 Break)))
              (:Completed
                (if (LocalVariables|GetbFoundLocation)
                  (Utilities|Array|RemoveIndex (LocalVariables|GettempLocations) (LocalVariables|GettempLocToRemove))
                  (goto _label Break))))))))))

(fn MakeEmptyDirection
  (bind _tempmap (LocalVariables|GettempMap))
  (Utilities|Map|Add _tempmap "" false)
  (Utilities|Map|Add _tempmap "NewEnumerator1" false)
  (Utilities|Map|Add _tempmap "NewEnumerator2" false)
  (Utilities|Map|Add _tempmap "NewEnumerator3" false)
  (return (LocalVariables|GettempMap)))

(fn AddTiletoLayout
  (params (AtLocation :type Vector%202D%20Structure%20%28by%20ref%29) (TileType :type ETileType%20Enum :default "NewEnumerator0") (ConnectionLocation :type Vector%202D%20Structure))
  (Utilities|Map|Add (Variables|References|GetTileLayout) AtLocation (Utilities|Struct|MakeSTileInformation TileType (Utility|MakeEmptyDirection)))
  (Layout|ConnectTiles ConnectionLocation AtLocation (Utility|WhereAmIComingfrom ConnectionLocation AtLocation)))

(fn GenerateReplacementTileLayout
  (bind _keys (Utilities|Map|Keys (Variables|References|GetTileLayout)))
  ;[1 1 1] make sure have replacement tiles
  (LocalVariables|SettemptLayout _keys)
  (if (> (Utilities|Array|Length (Variables|Metrics|GetReplacementTiles)) 0)
    (bind _arrayelement (Utilities|Array|ReverseforEachLoop (Variables|Metrics|GetReplacementTiles))
      (:LoopBody
        ;[1 1 1] if we do we check ever generic tile in the layout if their directions match replacing them with each other
        (bind _array_element (Utilities|Array|ForEachLoopwithBreak (LocalVariables|GettemptLayout) :!label _label)
          (:LoopBody
            (if (Utilities|Enum|Equal(Enum) (.Type (Utilities|Struct|BreakSTileInformation (.Value (Utilities|Map|Find (Variables|References|GetTileLayout) _array_element)))) "NewEnumerator0")
              (if (Utility|AreConnectionsMatching (.Directions (Utilities|Struct|BreakSTileInformation (.Value (Utilities|Map|Find (Variables|References|GetTileLayout) _array_element)))) (.TileConnection (Utilities|GetClassDefaults _arrayelement)))
                (Utilities|Map|Add (Variables|References|GetTileLayout) _array_element (Utilities|Struct|MakeSTileInformation "NewEnumerator4" (.TileConnection (Utilities|GetClassDefaults _arrayelement))))
                (Utilities|Map|Add (Variables|References|GetReplacedTileClass) _array_element _arrayelement)
                (goto _label Break)))))))))

(fn AddStartTiletoLayout
  (Utilities|Map|Add :TargetMap (Variables|References|GetTileLayout) :Value (Utilities|Struct|MakeSTileInformation "NewEnumerator1" (Utility|MakeEmptyDirection))))

(fn TryAddTiletoLayout
  (params (StartingLocation :type Vector%202D%20Structure) (WantedDirection :type ECardinalPoint%20Enum :default "NewEnumerator0") (TileType :type ETileType%20Enum :default "NewEnumerator0"))
  (bind (_foundlocation _tocardinal) (Rules|FindRandomNextLocation StartingLocation WantedDirection))
  (if (Utilities|Enum|NotEqual(Enum) _tocardinal "NewEnumerator4")
    (Layout|AddTiletoLayout _foundlocation TileType StartingLocation)
    (return true _foundlocation)
    (else
      (return false ""))))

(fn AddEndTiletoLayout
  (params (StartingLocation :type Vector%202D%20Structure))
  (bind (_foundlocation _tocardinal) (Rules|FindRandomNextLocation StartingLocation "NewEnumerator4"))
  (Utilities|Map|Add (Variables|References|GetTileLayout) _foundlocation (Utilities|Struct|MakeSTileInformation "NewEnumerator2" (Utility|MakeEmptyDirection)))
  (Layout|ConnectTiles StartingLocation _foundlocation (Utility|RevertCardinal _tocardinal)))

(fn StepBack
  (params (WantedDirection :type ECardinalPoint%20Enum :default "NewEnumerator0") (TileType :type ETileType%20Enum :default "NewEnumerator0"))
  ;[1 1 1] step back is a temp variable used to steo back each time we find ourselves incapable of adding more tiles
  (LocalVariables|SetstepBack 0)
  (Math|Integer|IncrementInt (LocalVariables|GetstepBack) :!label _label
    (:%20%20
      (bind _keys (Utilities|Map|Keys (Variables|References|GetTileLayout)))
      ;[1 1 1] trying to add new tile from previous location
      (bind _output_get (LocalVariables|SetpreviousLocation (LocalVariables|GetpreviousLocation)))
      (bind (_succesfullyadded _foundlocation) (Layout|TryAddTiletoLayout _output_get WantedDirection TileType))
      (if _succesfullyadded
        (return _foundlocation)
        (else
          (goto _label))))))

(fn ShouldStepBack
  (params (TileIndex :type Integer))
  (if (!= TileIndex 1)
    (return (< (Math|Random|RandomFloatinRange 1.0 1e+02) (Variables|Metrics|GetStepBackChance)))
    (else
      (return false))))

(fn CalculateStepstoStart
  (bind _keys (Utilities|Map|Keys (Variables|References|GetTileLayout)))
  (for (_array_element _array_index) _keys
    (LocalVariables|SetCurrentTile _array_element)
    (LocalVariables|SettempStepsToStart _array_index)
    (for _array_element_2 (Utility|GetLocationsAround (LocalVariables|GetCurrentTile))
      (if (Utility|IsLocationUsed _array_element_2)
        (if (Utility|AreTilesConnected _array_element_2 (LocalVariables|GetCurrentTile))
          _)))))