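; Dungeon Blueprint holding early, unfinished logic for random room placement in a square maze area.
; GenerateRoom picks a random size and a position that fits within MazeSize, with the room size limits wired reversed into Min and Max.
; TryPlacingARoom tests that candidate against stored rooms but returns inside the loop, after the first one.
; The overlap check is a stub returning false, and no event or construction logic starts generation.
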(event EventBeginPlay)

(event Collision|EventActorBeginOverlap
  (params (OtherActor :type Actor%20Object%20Reference)))

(event EventTick
  (params (DeltaSeconds :type Float%20%28single-precision%29)))

(fn ConstructionScript)

(fn GenerateRoom
  (LocalVariables|SetSize (Math|Vector|MakeVector (Math|Conversions|ToFloat(Integer) (Math|Random|RandomIntegerinRange (Variables|Default|GetMaxRoomSize) (Variables|Default|GetMinRoomSize))) (Math|Conversions|ToFloat(Integer) (Math|Random|RandomIntegerinRange (Variables|Default|GetMaxRoomSize) (Variables|Default|GetMinRoomSize))) 0.0))
  (LocalVariables|SetPosition (Math|Vector|MakeVector (Math|Conversions|ToFloat(Integer) (Math|Random|RandomIntegerinRange 0 (- (Variables|Default|GetMazeSize) (Math|Float|Truncate (.X (Math|Vector|BreakVector (LocalVariables|GetSize))))))) (Math|Conversions|ToFloat(Integer) (Math|Random|RandomIntegerinRange 0 (- (Variables|Default|GetMazeSize) (Math|Float|Truncate (.Y (Math|Vector|BreakVector (LocalVariables|GetSize))))))) 0.0))
  (return (LocalVariables|GetPosition) (LocalVariables|GetSize)))

(fn TryPlacingARoom
  (bind (_newposition _newsize) (CallFunction|GenerateRoom))
  (LocalVariables|SetRoomPos _newposition)
  (LocalVariables|SetRoomSize _newsize)
  (for (_array_element _array_index) (Variables|Default|GetRoomPositions)
    (bind _overlap (CallFunction|OverlappingRoom? _array_element (Utilities|Array|Get(acopy) (Variables|Default|GetRoomSizes) _array_index) (LocalVariables|GetRoomPos) (LocalVariables|GetRoomSize)))
    (LocalVariables|SetNotOverlapping (and (not _overlap) (LocalVariables|GetNotOverlapping)))
    (return (LocalVariables|GetNotOverlapping) (LocalVariables|GetRoomPos) (LocalVariables|GetRoomSize))))

(fn OverlappingRoom?
  (params (Room1Pos :type Vector) (Room1Size :type Vector) (Room2Pos :type Vector) (Room2Size :type Vector))
  (return false))